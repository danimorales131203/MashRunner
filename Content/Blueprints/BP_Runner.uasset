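; BP_Runner is a flipbook-sprite character that constantly moves along +X, with speed driven by alternately tapping left and right power inputs.
; Each alternating tap raises max walk speed up to a cap, while Tick drains it, both scaled by velocity-sampled ramps.
; Velocity selects the idle or run flipbook and sets run playback rate.
; A resettable DoOnce plays footstep sounds on two run frames.
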(event Input|EnhancedActionEvents|EnhancedInputActionIA_Powerleft
  (params (ActionValue :type Boolean) (ElapsedSeconds :type Float%20%28double-precision%29) (TriggeredSeconds :type Float%20%28double-precision%29) (InputAction :type Input%20Action%20Object%20Reference :default "/Game/Input/Actions/IA_Powerleft.IA_Powerleft"))
  (:Started
    (if (Utilities|Enum|NotEqual(Enum) (Variables|Default|GetLastInput) "NewEnumerator1")
      (Variables|Default|SetLastInput "NewEnumerator1")
      (CallFunction|IncreaseSpeed))))

(event Input|EnhancedActionEvents|EnhancedInputActionIA_Powerright
  (params (ActionValue :type Boolean) (ElapsedSeconds :type Float%20%28double-precision%29) (TriggeredSeconds :type Float%20%28double-precision%29) (InputAction :type Input%20Action%20Object%20Reference :default "/Game/Input/Actions/IA_Powerright.IA_Powerright"))
  (:Started
    (if (Utilities|Enum|NotEqual(Enum) (Variables|Default|GetLastInput) "NewEnumerator2")
      (Variables|Default|SetLastInput "NewEnumerator2")
      (CallFunction|IncreaseSpeed))))

(event EventBeginPlay
  (bind _asplayer_controller (Utilities|Casting|CastToPlayerController (Pawn|GetController)))
  (Input|AddMappingContext (PlayerController|LocalPlayerSubsystems|GetEnhancedInputLocalPlayerSubsystem _asplayer_controller) "/Game/Input/IMC_Runner.IMC_Runner" 0 "(bIgnoreAllPressedKeysUntilRelease=True,bForceImmediately=False,bNotifyUserSettings=False)"))

(event Collision|EventActorBeginOverlap
  (params (OtherActor :type Actor%20Object%20Reference)))

(event EventTick
  (params (DeltaSeconds :type Float%20%28single-precision%29))
  (bind _sprite (Variables|Default|GetSprite))
  (bind _returnvalue (Class|PaperFlipbookComponent|GetPlaybackPositioninFrames _sprite))
  (Pawn|Input|AddMovementInput "1.000000,0.000000,0.000000" 1.0 false)
  (CallFunction|DecreaseSpeed DeltaSeconds)
  (CallFunction|UpdateFlipBook)
  (CallFunction|SetRunPlayrate)
  (if (== (Class|PaperFlipbookComponent|GetFlipbook (Variables|Default|GetSprite)) "/Game/PaperAssets/Runner/FB_Speed_Run.FB_Speed_Run")
    (if (or (== _returnvalue 1) (== _returnvalue 5))
      (Utilities|FlowControl|DoOnce false :!label _label
        (:Completed
          (Audio|PlaySound2D "/Game/Sounds/Footsteps/Cue_FootStep.Cue_FootStep" 1.0 1.0 0.0 0 0)))
      (else
        (goto _label Reset)))))

(fn ConstructionScript)

(fn IncreaseSpeed
  (Variables|/Script/Engine.CharacterMovementComponent|SetMaxWalkSpeed (Variables|Character|GetCharacterMovement) (Math|Float|Clamp(Float) (+ (Variables|/Script/Engine.CharacterMovementComponent|GetMaxWalkSpeed (Variables|Character|GetCharacterMovement)) (* (Variables|Default|GetSpeedIncreasePerTap) (Math|Curves|GetFloatValue (Variables|Default|GetSpeedIncreaseRamp) (Math|Vector|VectorLength (Variables|/Script/Engine.MovementComponent|GetVelocity (Variables|Character|GetCharacterMovement)))))) 0.0 (Variables|Default|GetMaxSpeed))))

(fn DecreaseSpeed
  (params (Delta%20Seconds :type Float%20%28double-precision%29))
  (Variables|/Script/Engine.CharacterMovementComponent|SetMaxWalkSpeed (Variables|Character|GetCharacterMovement) (Math|Float|Max(Float) (- (Variables|/Script/Engine.CharacterMovementComponent|GetMaxWalkSpeed (Variables|Character|GetCharacterMovement)) (* Delta%20Seconds (* (Variables|Default|GetSlowMult) (Math|Curves|GetFloatValue (Variables|Default|GetSpeedDecreaseRamp) (Math|Vector|VectorLength (Variables|/Script/Engine.MovementComponent|GetVelocity (Variables|Character|GetCharacterMovement))))))) 0.0)))

(fn UpdateFlipBook
  (Sprite|SetFlipbook (Variables|Default|GetSprite) (select (> (Math|Vector|VectorLength (Variables|/Script/Engine.MovementComponent|GetVelocity (Variables|Character|GetCharacterMovement))) 0.0) "/Game/PaperAssets/Runner/FB_Speed_Run.FB_Speed_Run" "/Game/PaperAssets/Runner/FB_Speed_Idle.FB_Speed_Idle")))

(fn SetRunPlayrate
  (if (== (Class|PaperFlipbookComponent|GetFlipbook (Variables|Default|GetSprite)) "/Game/PaperAssets/Runner/FB_Speed_Run.FB_Speed_Run")
    (Components|Timeline|SetPlayRate (Variables|Default|GetSprite) (/ (Math|Vector|VectorLength (Variables|/Script/Engine.MovementComponent|GetVelocity (Variables|Character|GetCharacterMovement))) (Variables|Default|GetMaxSpeed)))
    (else
      (Components|Timeline|SetPlayRate (Variables|Default|GetSprite) 1.0))))